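; BP_InfoBlock is a trigger block that shows an info popup while the custom third-person character overlaps its Box.
; Begin overlap creates W_InfoPopup with SampleText, and end overlap removes it.
; When the Soup flag is set, a short delay leads to a party horn and replaces the popup with a W_Soup widget, which is removed after a longer delay.
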(event OnComponentBeginOverlap(Box)
  (params (OverlappedComponent :type Primitive%20Component%20Object%20Reference) (OtherActor :type Actor%20Object%20Reference) (OtherComp :type Primitive%20Component%20Object%20Reference) (OtherBodyIndex :type Integer) (bFromSweep :type Boolean) (SweepResult :type Hit%20Result%20Structure%20%28by%20ref%29))
  (Utilities|Casting|CastToBP_ThirdPersonCharacterCustom OtherActor)
  (bind _returnvalue (UserInterface|CreateWidget "/Game/Widgets/W_InfoPopup.W_InfoPopup_C"))
  (Variables|/Script/UMG.TextBlock|SetText (Variables|/Game/Widgets/W_InfoPopup.W_InfoPopup_C|GetInfo _returnvalue) (Variables|Default|GetSampleText))
  (UserInterface|Viewport|AddtoViewport _returnvalue 0)
  (if (Variables|Default|GetSoup)
    (Utilities|FlowControl|Delay 2.0)
    (Audio|PlaySound2D "/Game/Audio/PartyHorn_Cue.PartyHorn_Cue" 1.0 1.0 0.0 0 0)
    (Widget|RemovefromParent _returnvalue)
    (bind _returnvalue_2 (UserInterface|CreateWidget "/Game/Widgets/W_Soup.W_Soup_C"))
    (UserInterface|Viewport|AddtoViewport _returnvalue_2 0)
    (Utilities|FlowControl|Delay 1e+01)
    (Widget|RemovefromParent _returnvalue_2)))

(event OnComponentEndOverlap(Box)
  (params (OverlappedComponent :type Primitive%20Component%20Object%20Reference) (OtherActor :type Actor%20Object%20Reference) (OtherComp :type Primitive%20Component%20Object%20Reference) (OtherBodyIndex :type Integer))
  (Utilities|Casting|CastToBP_ThirdPersonCharacterCustom OtherActor)
  (Widget|RemovefromParent (stale OnComponentBeginOverlap(Box) _returnvalue)))

(fn ConstructionScript)