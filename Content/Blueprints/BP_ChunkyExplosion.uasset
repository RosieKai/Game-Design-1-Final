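; BP_ChunkyExplosion is an explosion effect actor that plays a Niagara system.
; On BeginPlay it enables player 0 input and stores the location of the BP_ThirdPersonCharacterCustom actor.
; Its Boom event teleports the actor to that stored location, which is not refreshed afterward, and activates the effect.
; A debug E key activates Niagara in place.
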(event Custom|Boom
  (Transformation|Teleport (Variables|Default|GetPlayerLocation) "0, 0, 0")
  (Components|Activation|Activate (Variables|Default|GetNiagara) false))

(event EventBeginPlay
  (Input|EnableInput (Game|GetPlayerController 0))
  (bind _returnvalue (Actor|GetActorOfClass "/Game/Blueprints/BP_ThirdPersonCharacterCustom.BP_ThirdPersonCharacterCustom_C"))
  (Variables|Default|SetPlayerLocation (Transformation|GetActorLocation _returnvalue)))

(event Collision|EventActorBeginOverlap
  (params (OtherActor :type Actor%20Object%20Reference)))

(event EventTick
  (params (DeltaSeconds :type Float%20%28single-precision%29)))

(event Input|KeyboardEvents|DebugKeyE
  (params (Key :type Key%20Structure :default "None") (ActionValue :type Input%20Action%20Value%20Structure))
  (:Pressed
    (Components|Activation|Activate (Variables|Default|GetNiagara) false)))

(fn ConstructionScript)