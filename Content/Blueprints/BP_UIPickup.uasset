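; BP_UIPickup is an actor that shows a floating W_UIPickup label with its own display name.
; On BeginPlay it creates the widget, assigns it to its Widget component and sets the ItemName text.
; FacePlayer turns that component toward the player camera, re-calling itself through a short Delay instead of using Tick.
; No overlap or pickup logic is implemented here.
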(event Custom|FacePlayer
  (Transformation|SetWorldRotation (Variables|Default|GetWidget) (Math|Rotator|FindLookatRotation (Transformation|GetWorldLocation (Variables|Default|GetWidget)) (Transformation|GetWorldLocation (Variables|/Script/Engine.Actor|GetRootComponent (Game|GetPlayerCameraManager 0)))) false false)
  (Utilities|FlowControl|Delay 0.1)
  (CallFunction|FacePlayer))

(event EventBeginPlay
  (CallFunction|FacePlayer)
  (bind _returnvalue (UserInterface|CreateWidget "/Game/Widgets/W_UIPickup.W_UIPickup_C"))
  (UserInterface|SetWidget (Variables|Default|GetWidget) _returnvalue)
  (Variables|/Script/UMG.TextBlock|SetText (Variables|/Game/Widgets/W_UIPickup.W_UIPickup_C|GetItemName _returnvalue) (Utilities|Text|ToText(String) (Utilities|GetDisplayName self))))

(event Collision|EventActorBeginOverlap
  (params (OtherActor :type Actor%20Object%20Reference)))

(event EventTick
  (params (DeltaSeconds :type Float%20%28single-precision%29)))

(fn ConstructionScript)