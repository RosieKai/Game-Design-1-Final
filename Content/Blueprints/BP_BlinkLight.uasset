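; BP_BlinkLight is an actor that blinks a sphere by swapping its material between grey and blue light.
; From BeginPlay, ChangeLightStage switches on a Stage counter, then calls itself again after a one-second delay, forming an endless loop.
; The first two stages show grey and advance the counter, while the third shows blue and resets it.
; An unexpected stage only prints a debug string, ending the loop.
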(event Custom|ChangeLightStage
  (switch int (Variables|Default|GetStage)
    (:Default
      (Development|PrintString "Hello"))
    (:0
      (Rendering|Material|SetMaterial (Variables|Default|GetSphere) 0 "/Game/Materials/MI_Grey.MI_Grey" :!label _label)
      (Variables|Default|SetStage (+ (Variables|Default|GetStage) 1))
      (Utilities|FlowControl|Delay 1.0 :!label _label_2)
      (CallFunction|ChangeLightStage))
    (:1
      (goto _label))
    (:2
      (Rendering|Material|SetMaterial (Variables|Default|GetSphere) 0 "/Game/Materials/MI_BlueLight.MI_BlueLight")
      (Variables|Default|SetStage 0)
      (goto _label_2))))

(event EventBeginPlay
  (CallFunction|ChangeLightStage))

(fn ConstructionScript)