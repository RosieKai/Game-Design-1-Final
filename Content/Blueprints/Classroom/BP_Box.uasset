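; BP_Box is an interactive classroom puzzle checker that opens the main menu when the desk answers total 18.
; On BeginPlay it counts circle, triangle and diamond actors, sets each count-matched desk's answer shape by row, and starts a ticking clock sound.
; Its overlap trigger shows an info prompt and registers itself with the player character.
; Change, effective only in range, adds each desk's Huh value to a running, never-reset tally.
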(event OnComponentBeginOverlap(Btn_Coll)
  (params (OverlappedComponent :type Primitive%20Component%20Object%20Reference) (OtherActor :type Actor%20Object%20Reference) (OtherComp :type Primitive%20Component%20Object%20Reference) (OtherBodyIndex :type Integer) (bFromSweep :type Boolean) (SweepResult :type Hit%20Result%20Structure%20%28by%20ref%29))
  (Rendering|SetVisibility (Variables|Default|GetInfo) true false)
  (Variables|Default|Setrange true)
  (bind _asbp_third_person_character_custom (Utilities|Casting|CastToBP_ThirdPersonCharacterCustom OtherActor))
  (Variables|/Game/Blueprints/BP_ThirdPersonCharacterCustom.BP_ThirdPersonCharacterCustom_C|SetWhichDesk _asbp_third_person_character_custom self))

(event OnComponentEndOverlap(Btn_Coll)
  (params (OverlappedComponent :type Primitive%20Component%20Object%20Reference) (OtherActor :type Actor%20Object%20Reference) (OtherComp :type Primitive%20Component%20Object%20Reference) (OtherBodyIndex :type Integer))
  (Rendering|SetVisibility (Variables|Default|GetInfo) false false)
  (Variables|Default|Setrange false))

(event EventBeginPlay
  (Utilities|FlowControl|Delay 0.005)
  (bind _outactors (Actor|GetAllActorsOfClass "/Game/Blueprints/Classroom/BP_Circle.BP_Circle_C"))
  (Variables|Default|SetCirc (Utilities|Array|Length _outactors))
  (bind _outactors_2 (Actor|GetAllActorsOfClass "/Game/Blueprints/Classroom/BP_Triangle.BP_Triangle_C"))
  (Variables|Default|SetTri (Utilities|Array|Length _outactors_2))
  (bind _outactors_3 (Actor|GetAllActorsOfClass "/Game/Blueprints/Classroom/BP_Diamond.BP_Diamond_C"))
  (Variables|Default|SetDiam (Utilities|Array|Length _outactors_3))
  (bind _outactors_4 (Actor|GetAllActorsOfClass "/Game/Blueprints/Classroom/BP_Desk.BP_Desk_C"))
  (for _array_element _outactors_4
    (switch int (Variables|/Game/Blueprints/Classroom/BP_Desk.BP_Desk_C|GetRow _array_element)
      (:Default
        (Development|PrintString "Oopsies" :!label _label))
      (:0
        (goto _label))
      (:1
        (if (== (Variables|/Game/Blueprints/Classroom/BP_Desk.BP_Desk_C|GetColumn _array_element) (Variables|Default|GetCirc))
          (Variables|/Game/Blueprints/Classroom/BP_Desk.BP_Desk_C|SetShapeAns _array_element "NewEnumerator0")))
      (:2
        (if (== (Variables|/Game/Blueprints/Classroom/BP_Desk.BP_Desk_C|GetColumn _array_element) (Variables|Default|GetTri))
          (Variables|/Game/Blueprints/Classroom/BP_Desk.BP_Desk_C|SetShapeAns _array_element "NewEnumerator1")))
      (:3
        (if (== (Variables|/Game/Blueprints/Classroom/BP_Desk.BP_Desk_C|GetColumn _array_element) (Variables|Default|GetDiam))
          (Variables|/Game/Blueprints/Classroom/BP_Desk.BP_Desk_C|SetShapeAns _array_element "NewEnumerator2")))))
  (bind _returnvalue (Audio|SpawnSoundatLocation "/Game/Audio/Whispers/clock-ticking-natural-room-verb-17249.clock-ticking-natural-room-verb-17249" (Transformation|GetWorldLocation (Variables|Default|GetCube)) "0, 0, 0" 1.0 1.0 0.0 0 0))
  (Utilities|FlowControl|Delay 5.0)
  (Audio|Components|Audio|AdjustVolume _returnvalue 17.0 5.0 "Logarithmic" :!class /Script/Engine.AudioComponent))

(event EventChange
  (if (Variables|Default|Getrange)
    (bind _outactors (Actor|GetAllActorsOfClass "/Game/Blueprints/Classroom/BP_Desk.BP_Desk_C"))
    (for _array_element _outactors
      (Variables|Default|SetAnsCount (+ (Variables|/Game/Blueprints/Classroom/BP_Desk.BP_Desk_C|Gethuh _array_element) (Variables|Default|GetAnsCount)))
      (if (== (Variables|Default|GetAnsCount) 18)
        (Game|OpenLevel(byObjectReference) "/Game/Maps/MainMenu.MainMenu")))))

(fn ConstructionScript)

(fn AddTally)