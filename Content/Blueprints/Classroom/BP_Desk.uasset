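; Classroom puzzle desk where the player cycles a displayed shape to match the desk's answer.
; Overlapping its collision shows a press prompt, sets InRange and registers the desk as the character's WhichDesk.
; When in range, Change destroys and spawns shape actors at ShapeZone, cycling circle, triangle, diamond and empty.
; Each change compares against ShapeAns to set Correct and a Huh flag, which also starts set when the answer is empty.
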(event OnComponentBeginOverlap(Collision)
  (params (OverlappedComponent :type Primitive%20Component%20Object%20Reference) (OtherActor :type Actor%20Object%20Reference) (OtherComp :type Primitive%20Component%20Object%20Reference) (OtherBodyIndex :type Integer) (bFromSweep :type Boolean) (SweepResult :type Hit%20Result%20Structure%20%28by%20ref%29))
  (Rendering|SetVisibility (Variables|Default|GetPressTXT) true false)
  (Variables|Default|SetInRange true)
  (bind _asbp_third_person_character_custom (Utilities|Casting|CastToBP_ThirdPersonCharacterCustom OtherActor))
  (Variables|/Game/Blueprints/BP_ThirdPersonCharacterCustom.BP_ThirdPersonCharacterCustom_C|SetWhichDesk _asbp_third_person_character_custom self))

(event OnComponentEndOverlap(Collision)
  (params (OverlappedComponent :type Primitive%20Component%20Object%20Reference) (OtherActor :type Actor%20Object%20Reference) (OtherComp :type Primitive%20Component%20Object%20Reference) (OtherBodyIndex :type Integer))
  (if (== OtherActor "/Game/Blueprints/BP_ThirdPersonCharacterCustom.BP_ThirdPersonCharacterCustom")
    (Rendering|SetVisibility (Variables|Default|GetPressTXT) false false)
    (Variables|Default|SetInRange false)
    (Development|PrintString "Hello")))

(event EventBeginPlay
  (Rendering|SetVisibility (Variables|Default|GetPressTXT) false false)
  (Utilities|FlowControl|Delay 0.4)
  (if (== 3 (Variables|Default|GetShapeAns))
    (Variables|Default|Sethuh 1)))

(event EventChange
  (bind _shapezone (Variables|Default|GetShapeZone))
  (bind _returnvalue (Transformation|GetWorldTransform _shapezone))
  (if (Variables|Default|GetInRange)
    (switch Utilities|FlowControl|Switch|SwitchonE_Shape (Variables|Default|GetCurShape)
      (:NewEnumerator0
        (Actor|DestroyActor (stale _returnvalue_4))
        (bind _returnvalue_2 (Game|SpawnActorfromClass "/Game/Blueprints/Classroom/BP_Triangle.BP_Triangle_C" _returnvalue "Undefined" "MultiplyWithRoot" 0 0))
        (Variables|Default|SetCurShape "NewEnumerator1")
        (Variables|Default|SetCorrect (== 1 (Variables|Default|GetShapeAns))))
      (:NewEnumerator1
        (Actor|DestroyActor _returnvalue_2)
        (bind _returnvalue_3 (Game|SpawnActorfromClass "/Game/Blueprints/Classroom/BP_Diamond.BP_Diamond_C" _returnvalue "Undefined" "MultiplyWithRoot" 0 0))
        (Variables|Default|SetCurShape "NewEnumerator2")
        (Variables|Default|SetCorrect (== 2 (Variables|Default|GetShapeAns))))
      (:NewEnumerator2
        (Actor|DestroyActor _returnvalue_3)
        (Variables|Default|SetCurShape "NewEnumerator3")
        (Variables|Default|SetCorrect (== 3 (Variables|Default|GetShapeAns))))
      (:NewEnumerator3
        (bind _returnvalue_4 (Game|SpawnActorfromClass "/Game/Blueprints/Classroom/BP_Circle.BP_Circle_C" _returnvalue "Undefined" "MultiplyWithRoot" 0 0))
        (Variables|Default|SetCurShape "NewEnumerator0")
        (Variables|Default|SetCorrect (== 0 (Variables|Default|GetShapeAns)))))
    (if (Variables|Default|GetCorrect)
      (Variables|Default|Sethuh 1)
      (else
        (Variables|Default|Sethuh 0)))))

(event EventAddTally)

(fn ConstructionScript)