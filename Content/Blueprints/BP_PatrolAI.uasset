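; Patrol AI character that walks between actors tagged "PatrolPoint-test" at a randomized walk speed set on BeginPlay.
; Patrol loops through the shuffled points with AI MoveTo, advancing after success or failure and reshuffling after each full pass.
; A separate Attack loop chases the player and calls TakeDamage on BP_ThirdPersonCharacterCustom upon arrival, retrying after failures.
; Nothing in this graph calls Attack.
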(event Custom|Attack
  (bind _returnvalue (Game|GetPlayerCharacter 0))
  (AI|AIMoveTo self "0, 0, 0" _returnvalue 2e+02 false ; Move to player's location, stop 2 meters away.
    (:OnSuccess
      (Development|PrintString "Hello")
      (bind _asbp_third_person_character_custom (Utilities|Casting|CastToBP_ThirdPersonCharacterCustom _returnvalue))
      (Default|TakeDamage _asbp_third_person_character_custom)
      (Utilities|FlowControl|Delay 2.0))
    (:OnFail
      (Development|PrintString "Goodbye")
      (Utilities|FlowControl|Delay 1.0)))
  (CallFunction|Attack))

(event Custom|Patrol
  (AI|AIMoveTo self (Transformation|GetActorLocation (Utilities|Array|Get(acopy) (stale EventBeginPlay _outactors) (Variables|Default|GetNextPoint))) 0 2e+02 false ; Move to player's location, stop 2 meters away.
    (:OnSuccess
      _)
    (:OnFail
      _))
  (bind _result (Math|Integer|IncrementInt (Variables|Default|GetNextPoint))
    (:%20%20
      (if (>= _result (Utilities|Array|Length (stale EventBeginPlay _outactors)))
        (Variables|Default|SetNextPoint 0)
        (Utilities|Array|Shuffle (stale EventBeginPlay _outactors)))
      (Utilities|FlowControl|Delay 1.0)
      (CallFunction|Patrol))))

(event EventBeginPlay
  (bind _outactors (Actor|GetAllActorsOfClasswithTag "/Script/Engine.Actor" "PatrolPoint-test"))
  (Utilities|Array|Shuffle _outactors)
  (Variables|/Script/Engine.CharacterMovementComponent|SetMaxWalkSpeed (Variables|Character|GetCharacterMovement) (Math|Conversions|ToFloat(Integer) (* (Math|Random|RandomIntegerinRange 60 10) 20)))
  (CallFunction|Patrol))

(fn ConstructionScript)