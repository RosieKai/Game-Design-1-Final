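; BP_Counter is a pizza assembly station where the player builds a pizza from held ingredients.
; Overlapping its box reads the custom third-person character's held item and accepts dough, sauce, cheese and pepperoni only in that order, revealing each layer mesh and taking the item.
; Overlapping empty-handed once pepperoni is placed resets the counter, spawns a BP_Pizza and hands it to the player as an uncooked pizza.
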(event OnComponentBeginOverlap(Box)
  (params (OverlappedComponent :type Primitive%20Component%20Object%20Reference) (OtherActor :type Actor%20Object%20Reference) (OtherComp :type Primitive%20Component%20Object%20Reference) (OtherBodyIndex :type Integer) (bFromSweep :type Boolean) (SweepResult :type Hit%20Result%20Structure%20%28by%20ref%29))
  (bind _asbp_third_person_character_custom (Utilities|Casting|CastToBP_ThirdPersonCharacterCustom OtherActor))
  (Development|PrintString (Utilities|String|EnumtoString (Variables|/Game/Blueprints/BP_ThirdPersonCharacterCustom.BP_ThirdPersonCharacterCustom_C|GetItemHeld _asbp_third_person_character_custom)) true true "(R=0.084533,G=0.343750,B=0.073763,A=1.000000)")
  (switch Utilities|FlowControl|Switch|SwitchonE_PizzaItem (Variables|/Game/Blueprints/BP_ThirdPersonCharacterCustom.BP_ThirdPersonCharacterCustom_C|GetItemHeld _asbp_third_person_character_custom)
    (:NewEnumerator4
      (if (Variables|Default|GetPepparoni)
        (Variables|Default|Setdough false)
        (Variables|Default|SetSauce false)
        (Variables|Default|SetCheese false)
        (Variables|Default|SetPepparoni false)
        (Rendering|SetVisibility (Variables|Default|GetRolledDough) false false)
        (bind _returnvalue (Game|SpawnActorfromClass "/Game/Blueprints/PizzaPlace/BP_Pizza.BP_Pizza_C" (Math|Transform|MakeTransform "0, 0, 0") "Undefined" "MultiplyWithRoot" 0 0))
        (bind _asbp_third_person_character_custom_2 (Utilities|Casting|CastToBP_ThirdPersonCharacterCustom OtherActor))
        (Default|TrytoPickUp _asbp_third_person_character_custom_2 _returnvalue "NewEnumerator5")
        (else
          (Development|PrintString "You Aren't Holding Anything" true true "(R=0.232018,G=0.316761,B=0.360417,A=1.000000)"))))
    (:NewEnumerator0
      (if (Variables|Default|Getdough)
        (Development|PrintString "You Already Placed That" true true "(R=0.232018,G=0.316761,B=0.360417,A=1.000000)" :!label _label)
        (else
          (Variables|Default|Setdough true)
          (Rendering|SetVisibility (Variables|Default|GetRolledDough) true false)
          (bind _asbp_third_person_character_custom_3 (Utilities|Casting|CastToBP_ThirdPersonCharacterCustom OtherActor :!label _label_2))
          (Default|SetItDown _asbp_third_person_character_custom_3))))
    (:NewEnumerator1
      (if (Variables|Default|GetSauce)
        (goto _label)
        (elif (Variables|Default|Getdough)
          (Variables|Default|SetSauce true)
          (Rendering|SetVisibility (Variables|Default|GetPlacedSauce) true false)
          (goto _label_2)
          (else
            (Development|PrintString "Not Yet Nerd" true true "(R=0.232018,G=0.316761,B=0.360417,A=1.000000)" :!label _label_3)))))
    (:NewEnumerator2
      (if (Variables|Default|GetCheese)
        (goto _label)
        (elif (Variables|Default|GetSauce)
          (Variables|Default|SetCheese true)
          (Rendering|SetVisibility (Variables|Default|GetPlacedCheese) true false)
          (goto _label_2)
          (else
            (goto _label_3)))))
    (:NewEnumerator3
      (if (Variables|Default|GetPepparoni)
        (goto _label)
        (elif (Variables|Default|GetCheese)
          (Variables|Default|SetPepparoni true)
          (Rendering|SetVisibility (Variables|Default|GetPlacedPep) true false)
          (goto _label_2)
          (else
            (goto _label_3)))))))

(event EventBeginPlay
  (Variables|Default|Setdough false)
  (Variables|Default|SetSauce false)
  (Variables|Default|SetCheese false)
  (Variables|Default|SetPepparoni false)
  (Rendering|SetVisibility (Variables|Default|GetRolledDough) false false))

(fn ConstructionScript)