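; Ducky is a PizzaPlace actor whose Ducky component moves and turns in an endless stepped cycle.
; On BeginPlay, the DUCKYTIME timeline drives its relative Y position and yaw from scaled move and turn tracks.
; When the timeline finishes, it folds the end values into stored offsets and replays after a short delay, so each cycle continues from the last pose.
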(event EventBeginPlay
  (Variables|Default|SetWorldRo 0.0)
  (Variables|Default|SetWorldLo 0.0)
  (bind (_direction _dukmove _dukturn) (Timeline|DUCKYTIME Play)
    (:Update
      (Transformation|SetRelativeLocationAndRotation (Variables|Default|GetDucky) (Math|Vector|MakeVector 0.0 (+ (* _dukmove 5e+02) (Variables|Default|GetWorldLo)) 0.0) (Math|Rotator|MakeRotator 0.0 0.0 (+ (* _dukturn 1.8e+02) (Variables|Default|GetWorldRo))) false false))
    (:Finished
      (Variables|Default|SetWorldLo (+ (* _dukmove 5e+02) (Variables|Default|GetWorldLo)))
      (Variables|Default|SetWorldRo (+ (* _dukturn 1.8e+02) (Variables|Default|GetWorldRo)))
      (Utilities|FlowControl|Delay 0.5)
      (Timeline|DUCKYTIME PlayFromStart))))

(event Collision|EventActorBeginOverlap
  (params (OtherActor :type Actor%20Object%20Reference)))

(event EventTick
  (params (DeltaSeconds :type Float%20%28single-precision%29)))

(fn ConstructionScript)