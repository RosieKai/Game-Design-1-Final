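; BP_Door2 is a locked door that consumes one key from the player character to open.
; Overlapping its collision unlocks it if KeyCount is positive, otherwise printing a refusal and playing a locked sound.
; A Timeline swings the door 90 degrees open with a sound, then reverses shortly after an overlap ends.
; Once unlocked it stays unlocked, reopening for any overlapping actor without another key.
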(event OnComponentBeginOverlap(Collision)
  (params (OverlappedComponent :type Primitive%20Component%20Object%20Reference) (OtherActor :type Actor%20Object%20Reference) (OtherComp :type Primitive%20Component%20Object%20Reference) (OtherBodyIndex :type Integer) (bFromSweep :type Boolean) (SweepResult :type Hit%20Result%20Structure%20%28by%20ref%29))
  (if (not (Variables|Default|GetDoorOpened))
    (if (Variables|Default|GetLocked)
      (bind _asbp_third_person_character_custom (Utilities|Casting|CastToBP_ThirdPersonCharacterCustom OtherActor))
      (if (> (Variables|/Game/Blueprints/BP_ThirdPersonCharacterCustom.BP_ThirdPersonCharacterCustom_C|GetKey%20Count _asbp_third_person_character_custom) 0) ; Like an If Statement
        (Variables|/Game/Blueprints/BP_ThirdPersonCharacterCustom.BP_ThirdPersonCharacterCustom_C|SetKey%20Count _asbp_third_person_character_custom (- (Variables|/Game/Blueprints/BP_ThirdPersonCharacterCustom.BP_ThirdPersonCharacterCustom_C|GetKey%20Count _asbp_third_person_character_custom) 1)) ; Remove a Key, then open door.
        (Variables|Default|SetLocked false)
        (Audio|PlaySoundatLocation "/Game/Audio/DoorOpens_Cue.DoorOpens_Cue" (Transformation|GetWorldLocation (Variables|Default|GetDefaultSceneRoot)) "0, 0, 0" 1.0 1.0 0.0 0 0 0 0 :!label _label)
        (Variables|Default|SetDoorOpened true)
        (bind _newtrack_0 (Timeline|Timeline PlayFromStart)
          (:Update
            (Transformation|SetRelativeRotation (Variables|Default|GetDoor) (Math|Rotator|MakeRotator 0.0 0.0 (* _newtrack_0 -9e+01)) false false)))
        (else
          (Development|PrintString "Where do you think you're going? Get back in the kitchen!" true true "(R=0.479167,G=0.051103,B=0.000000,A=1.000000)" 5.0)
          (Audio|PlaySoundatLocation "/Game/Audio/DoorLocked_Cue.DoorLocked_Cue" (Transformation|GetWorldLocation (Variables|Default|GetDefaultSceneRoot)) "0, 0, 0" 1.0 1.0 0.0 0 0 0 0)))
      (else
        (goto _label)))))

(event OnComponentEndOverlap(Collision)
  (params (OverlappedComponent :type Primitive%20Component%20Object%20Reference) (OtherActor :type Actor%20Object%20Reference) (OtherComp :type Primitive%20Component%20Object%20Reference) (OtherBodyIndex :type Integer))
  (Utilities|FlowControl|Delay 0.75)
  (if (Variables|Default|GetDoorOpened) ; Like an If Statement
    (Variables|Default|SetDoorOpened false)
    (bind _newtrack_0 (Timeline|Timeline ReverseFromEnd)
      (:Update
        (Transformation|SetRelativeRotation (Variables|Default|GetDoor) (Math|Rotator|MakeRotator 0.0 0.0 (* _newtrack_0 -9e+01)) false false)))))

(event EventBeginPlay
  (Variables|Default|SetLocked true)
  (Variables|Default|SetDoorOpened false))

(event Collision|EventActorBeginOverlap
  (params (OtherActor :type Actor%20Object%20Reference)))

(event EventTick
  (params (DeltaSeconds :type Float%20%28single-precision%29)))

(fn ConstructionScript)