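; Trigger volume that starts a "WitchTime" screen effect while the player character is inside, and sets off an explosion if they linger.
; BeginPlay finds the post-process volume tagged GlobalPPV and caches some of its settings.
; Entering plays a timeline that drives an Intensity setting and starts a four-second delay, then calls Boom on BP_ChunkyExplosion if StillThere remains set.
; Leaving clears that flag and writes back cached intensity and tint.
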(event OnComponentBeginOverlap(TriggerBox)
  (params (OverlappedComponent :type Primitive%20Component%20Object%20Reference) (OtherActor :type Actor%20Object%20Reference) (OtherComp :type Primitive%20Component%20Object%20Reference) (OtherBodyIndex :type Integer) (bFromSweep :type Boolean) (SweepResult :type Hit%20Result%20Structure%20%28by%20ref%29))
  (Utilities|Casting|CastToBP_ThirdPersonCharacterCustom OtherActor)
  (CallFunction|WitchTime))

(event OnComponentEndOverlap(TriggerBox)
  (params (OverlappedComponent :type Primitive%20Component%20Object%20Reference) (OtherActor :type Actor%20Object%20Reference) (OtherComp :type Primitive%20Component%20Object%20Reference) (OtherBodyIndex :type Integer))
  (Utilities|Casting|CastToBP_ThirdPersonCharacterCustom OtherActor)
  (CallFunction|EndWitchTime))

(event Custom|WitchTime
  (bind _globalppv (Variables|Default|GetGlobalPPV))
  (Utilities|FlowControl|Sequence
    (:then_0
      (bind _newtrack_0 (Timeline|Timeline PlayFromStart)
        (:Update
          (bind _structout (Utilities|Struct|SetmembersinPostProcessSettings (Variables|/Script/Engine.PostProcessVolume|GetSettings _globalppv) (* _newtrack_0 15.0)))
          (Variables|/Script/Engine.PostProcessVolume|SetSettings _globalppv _structout))))
    (:then_1
      (Variables|Default|SetStillThere true)
      (Utilities|FlowControl|Delay 4.0)
      (if (Variables|Default|GetStillThere)
        (bind _returnvalue (Actor|GetActorOfClass "/Game/Blueprints/BP_ChunkyExplosion.BP_ChunkyExplosion_C"))
        (Default|Boom _returnvalue)))))

(event Custom|EndWitchTime
  (bind _globalppv (Variables|Default|GetGlobalPPV))
  (bind _originalsettings (Variables|Default|GetOriginalSettings))
  (bind (_scenecolortint _scenefringeintensity) (Utilities|Struct|BreakPostProcessSettings _originalsettings))
  (Variables|Default|SetStillThere false)
  (bind _structout (Utilities|Struct|SetmembersinPostProcessSettings (Variables|/Script/Engine.PostProcessVolume|GetSettings _globalppv) _scenecolortint _scenefringeintensity))
  (Variables|/Script/Engine.PostProcessVolume|SetSettings _globalppv _structout))

(event EventBeginPlay
  (bind _outactors (Actor|GetAllActorsOfClasswithTag "/Script/Engine.PostProcessVolume" "GlobalPPV"))
  (bind _output_get (Variables|Default|SetGlobalPPV (Utilities|Array|Get(acopy) _outactors)))
  (Utilities|IsValid 0
    (:Is%20Valid
      (Development|PrintString "Loaded Global PPV")
      (Variables|Default|SetOriginalSettings (Utilities|Struct|MakePostProcessSettings (.SceneFringeIntensity (Utilities|Struct|BreakPostProcessSettings (Variables|/Script/Engine.PostProcessVolume|GetSettings _output_get))) (.AutoExposureBias (Utilities|Struct|BreakPostProcessSettings (Variables|/Script/Engine.PostProcessVolume|GetSettings _output_get))))))))

(fn ConstructionScript)